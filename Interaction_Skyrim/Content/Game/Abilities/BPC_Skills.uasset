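; Actor component that tracks available skill points and the rank of each assigned skill.
; Points can be awarded, queried and spent, independently of skill assignment.
; AssignSkill checks prerequisites and tier limits, raises the rank in a map, fires an update event and adds any linked ability to the player's BPC_Abilities.
; UnAssignSkill only lowers the rank, without notifying or removing abilities.
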(fn `AssignSkill`
  (params (skill :type "/Game/Game/UI/Data/DA_Skill Object Reference"))
  (bind _skill (`local.skill`))
  (bind (_value _returnvalue) (`BlueprintMapLibrary.Map_Find` (`self.SkillsAssigned`) (`local.skill`)))
  (bind _allmet (`/Game/Game/UI/Data/DA_Skill.ArePrerqMet` skill self))
  (if (and _allmet (<= (+ (`BlueprintMapLibrary.Map_Find` (`self.SkillsAssigned`) _skill) 1) (`/Game/Game/UI/Data/DA_Skill.GetNumberOfTiers` _skill)))
    (`BlueprintMapLibrary.Map_Add` (`self.SkillsAssigned`) (`local.skill`) (`KismetMathLibrary.SelectInt` (+ _value 1) 1 _returnvalue))
    (`self.OnSkillsUpdate`)
    ; Abilities are owned by the player
    (bind _ability (`/Game/Game/UI/Data/DA_Skill.Ability` (`local.skill`))
      (:`then`
        (bind _player (message `/Game/Game/player/interface/BPI_Player.GetPlayer` (`GameplayStatics.GetPlayerCharacter` 0)))
        (`/Game/Game/player/components/BPC_Abilities.AddAbility` (`Actor.GetComponentByClass` _player "/Game/Game/player/components/BPC_Abilities.BPC_Abilities_C") _ability))
      (:`else`))))

(fn `AwardSkillPoint`
  (params (skillPoint :type Integer))
  (set `self.skillPointsAvailable` (+ (`self.skillPointsAvailable`) skillPoint)))

(fn `QuerySkill`
  (params (skill :type "/Game/Game/UI/Data/DA_Skill Object Reference"))
  (returns (rank :type Integer) (return :type Boolean))
  (bind (_value _returnvalue) (`BlueprintMapLibrary.Map_Find` (`self.SkillsAssigned`) skill))
  (return _value _returnvalue))

(fn `QuerySkillPoints`
  (params (Query :type Integer))
  (returns (Return :type Boolean))
  (return (>= (`self.skillPointsAvailable`) Query)))

(fn `SpendSkillPoint`
  (params (Amount :type Integer))
  (bind _return (`self.QuerySkillPoints` Amount))
  (if _return
    (set `self.skillPointsAvailable` (- (`self.skillPointsAvailable`) Amount))))

(fn `UnAssignSkill`
  (params (skill :type "/Game/Game/UI/Data/DA_Skill Object Reference"))
  (if (> (`self.QuerySkill` skill) 0)
    (`BlueprintMapLibrary.Map_Add` (`self.SkillsAssigned`) skill (- (`BlueprintMapLibrary.Map_Find` (`self.SkillsAssigned`) (`local.skill`)) 1))))
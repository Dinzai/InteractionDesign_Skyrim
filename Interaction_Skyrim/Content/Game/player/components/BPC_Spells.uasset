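; Player component that shows and hides a spell effect when the owning player casts.
; On BeginPlay it gets the owner's PlayerMessage object and binds its Spell event to that object's OnSpellCast dispatcher.
; When casting turns on, it teleports TheSystem to the SpellEffectLocation's world position and activates it.
; When casting turns off, it deactivates the system.
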(event `self.ReceiveBeginPlay`
  (bind _player (message `/Game/Game/player/interface/BPI_Player.GetPlayer` (`self.GetOwner`)))
  (add `/Game/Game/player/BP_PlayerCharacter.On_Spell_Cast` _player (delegate `Spell`)))

(event `Spell`
  (params (isOn :type Boolean))
  (bind _thesystem (`self.theSystem`))
  (if isOn
    (`SceneComponent.K2_SetWorldLocation` _thesystem (`SceneComponent.K2_GetComponentLocation` (`/Game/Game/player/BP_PlayerCharacter.SpellEffectLocation` (stale `self.ReceiveBeginPlay` _player))) false true)
    (`self.Activate` _thesystem false)
    (else
      (`self.Deactivate` _thesystem))))
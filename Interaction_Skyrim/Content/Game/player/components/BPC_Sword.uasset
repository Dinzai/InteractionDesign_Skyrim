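; Player component that represents an equipped sword, with its lifetime matching the equip state.
; On BeginPlay it spawns a generic BP_AnyItem using the DA_Sword data asset and attaches it to the SwordSocket on the owner's skeletal mesh.
; It signals equip and unequip and switches the Skill value through the owner's PlayerMessage.
; RemoveSword reverts that state, then destroys the sword actor and the component itself.
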(event `self.ReceiveBeginPlay`
  (bind _player (message `/Game/Game/player/interface/BPI_Player.GetPlayer` (`self.GetOwner`)))
  (bind _returnvalue (`|SpawnActorFromClass` "/Game/Game/Items/Placeholder/BP_AnyItem.BP_AnyItem_C" (`KismetMathLibrary.MakeTransform` (0.0 0.0 0.0)) "AlwaysSpawn" "MultiplyWithRoot" null "/Game/Game/Items/Data/ItemData/DA_Sword.DA_Sword" null))
  (set `self.sword` _returnvalue)
  (`Actor.K2_AttachToComponent` _returnvalue (`/Game/Game/player/BP_PlayerCharacter.SkeletalMesh` _player) "SwordSocket" "SnapToTarget" "KeepWorld" "KeepWorld" true)
  (`/Game/Game/player/BP_PlayerCharacter.on_Sword_Equip` _player true)
  (set `/Game/Game/player/BP_PlayerCharacter.skill` 1 _player))

(event `RemoveSword`
  (bind _player (message `/Game/Game/player/interface/BPI_Player.GetPlayer` (`self.GetOwner`)))
  (set `/Game/Game/player/BP_PlayerCharacter.skill` 2 _player)
  (`/Game/Game/player/BP_PlayerCharacter.on_Sword_Equip` _player false)
  (`Actor.K2_DestroyActor` (`self.sword`))
  (`self.K2_DestroyComponent`))
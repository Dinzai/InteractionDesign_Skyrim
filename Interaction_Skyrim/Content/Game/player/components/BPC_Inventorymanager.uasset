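; Player inventory component that stores items in separate weapon, potion and misc arrays.
; Type-switch functions route an item to the matching add, remove or size function.
; Adds notify the player's message object to update that category's UI, plus an "added" call when the category was empty.
; Removals delete matching entries by looping over the array and send no notification; misc removal also prints a debug string.
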(fn `AddMiscItem`
  (params (misc :type "/Game/Game/Items/Data/PDA_ItemData Object Reference"))
  (bind _returnvalue (`self.GetMiscLength`))
  (bind _player (message `/Game/Game/player/interface/BPI_Player.GetPlayer` (`GameplayStatics.GetPlayerCharacter` 0)))
  (`KismetArrayLibrary.Array_Add` (`self.Misc_Inventory`) misc)
  (if (== _returnvalue 0)
    (`/Game/Game/player/BP_PlayerCharacter.On_Misc_Added` _player misc)
    (`self.GetMiscLength`)
    (`/Game/Game/player/BP_PlayerCharacter.On_UI_MiscUpdate` _player)
    (else
      (`self.GetMiscLength`)
      (`/Game/Game/player/BP_PlayerCharacter.On_UI_MiscUpdate` _player))))

(fn `AddPotionItem`
  (params (potionItem :type "/Game/Game/Items/Data/PDA_ItemData Object Reference"))
  (bind _returnvalue (`self.GetPotionInvLength`))
  (bind _player (message `/Game/Game/player/interface/BPI_Player.GetPlayer` (`GameplayStatics.GetPlayerCharacter` 0)))
  (`KismetArrayLibrary.Array_Add` (`self.Potion_Inventroy`) potionItem)
  (if (== _returnvalue 0)
    (`/Game/Game/player/BP_PlayerCharacter.On_PotionAdded` _player potionItem)
    (`self.GetPotionInvLength`)
    (`/Game/Game/player/BP_PlayerCharacter.On_UI_PotionUpdate` _player)
    (else
      (`self.GetPotionInvLength`)
      (`/Game/Game/player/BP_PlayerCharacter.On_UI_PotionUpdate` _player))))

(fn `AddWeaponItem`
  (params (weaponItem :type "/Game/Game/Items/Data/PDA_ItemData Object Reference"))
  (bind _returnvalue (`self.GetWeaponInvLength`))
  (bind _player (message `/Game/Game/player/interface/BPI_Player.GetPlayer` (`GameplayStatics.GetPlayerCharacter` 0)))
  (`KismetArrayLibrary.Array_Add` (`self.Weapon_Inventory`) weaponItem)
  (if (== _returnvalue 0)
    (`/Game/Game/player/BP_PlayerCharacter.On_WeaponAdded` _player weaponItem)
    (`self.GetWeaponInvLength`)
    (`/Game/Game/player/BP_PlayerCharacter.On_UI_WeaponUpdate` _player)
    (else
      (`self.GetWeaponInvLength`)
      (`/Game/Game/player/BP_PlayerCharacter.On_UI_WeaponUpdate` _player))))

(fn `GetMiscLength`
  (returns (ReturnValue :type Integer))
  (return (`KismetArrayLibrary.Array_Length` (`self.Misc_Inventory`))))

(fn `GetPotionInvLength`
  (returns (ReturnValue :type Integer))
  (return (`KismetArrayLibrary.Array_Length` (`self.Potion_Inventroy`))))

(fn `GetWeaponInvLength`
  (returns (ReturnValue :type Integer))
  (return (`KismetArrayLibrary.Array_Length` (`self.Weapon_Inventory`))))

(fn `ReadTypeAndDecideForAddition`
  (params (item :type "/Game/Game/Items/Data/PDA_ItemData Object Reference"))
  (switch `/Game/Game/Items/Data/ITEM_TYPE` (`/Game/Game/Items/Data/PDA_ItemData.type` item)
    (:`NewEnumerator0`
      (`self.AddWeaponItem` item))
    (:`NewEnumerator1`
      (`self.AddPotionItem` item))
    (:`NewEnumerator2`
      (`self.AddMiscItem` item))))

(fn `ReadTypeAndDecideForRemoval`
  (params (itemType :type "/Game/Game/Items/Data/PDA_ItemData Object Reference"))
  (switch `/Game/Game/Items/Data/ITEM_TYPE` (`/Game/Game/Items/Data/PDA_ItemData.type` itemType)
    (:`NewEnumerator0`
      (`self.RemoveWeaponItem` itemType))
    (:`NewEnumerator1`
      (`self.RemovePotionItem` itemType))
    (:`NewEnumerator2`
      (`KismetSystemLibrary.PrintString` "Hello")
      (`self.RemoveMiscItem` itemType))))

(fn `ReadTypeAndDecideForSize`
  (params (itemType :type "/Game/Game/Items/Data/PDA_ItemData Object Reference"))
  (returns (ReturnValue :type Integer))
  (switch `/Game/Game/Items/Data/ITEM_TYPE` (`/Game/Game/Items/Data/PDA_ItemData.type` itemType)
    (:`NewEnumerator0`
      (bind _returnvalue (`self.GetWeaponInvLength`))
      (return _returnvalue))
    (:`NewEnumerator1`
      (bind _returnvalue_2 (`self.GetPotionInvLength`))
      (return _returnvalue_2))
    (:`NewEnumerator2`
      (bind _returnvalue_3 (`self.GetMiscLength`))
      (return _returnvalue_3))))

(fn `RemoveMiscItem`
  (params (item :type "/Game/Game/Items/Data/PDA_ItemData Object Reference"))
  (bind _misc_inventory (`self.Misc_Inventory`))
  (for (_array_element _array_index) _misc_inventory
    (if (== _array_element item)
      (`KismetArrayLibrary.Array_Remove` _misc_inventory _array_index))))

(fn `RemovePotionItem`
  (params (item :type "/Game/Game/Items/Data/PDA_ItemData Object Reference"))
  (bind _potion_inventroy (`self.Potion_Inventroy`))
  (for (_array_element _array_index) _potion_inventroy
    (if (== _array_element item)
      (`KismetArrayLibrary.Array_Remove` _potion_inventroy _array_index))))

(fn `RemoveWeaponItem`
  (params (item :type "/Game/Game/Items/Data/PDA_ItemData Object Reference"))
  (bind _weapon_inventory (`self.Weapon_Inventory`))
  (for (_array_element _array_index) _weapon_inventory
    (if (== _array_element item)
      (`KismetArrayLibrary.Array_Remove` _weapon_inventory _array_index))))
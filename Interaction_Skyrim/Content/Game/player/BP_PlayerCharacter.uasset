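; Player character Blueprint that turns Enhanced Input actions for move, look and jump into character actions.
; Move and look pass their 2D axis values to the BPCMove and BPCLook components, keeping that logic out of the character.
; Jump calls the built-in Jump and StopJumping on trigger and cancel.
; GetPlayer returns the character itself, and the construction script is empty.
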(event `EnhancedInput|/Game/Settings/Input/IA_Move`
  (params (ActionValue :type "Vector2D Structure") (ElapsedSeconds :type "Float (double-precision)") (TriggeredSeconds :type "Float (double-precision)") (InputAction :type "InputAction Object Reference" :default "/Game/Settings/Input/IA_Move.IA_Move"))
  (:`Triggered`
    (`/Game/Game/player/components/BPC_Move.Move` (`self.BPC_Move`) ActionValue_X ActionValue_Y)))

(event `EnhancedInput|/Game/Settings/Input/IA_Look`
  (params (ActionValue :type "Vector2D Structure") (ElapsedSeconds :type "Float (double-precision)") (TriggeredSeconds :type "Float (double-precision)") (InputAction :type "InputAction Object Reference" :default "/Game/Settings/Input/IA_Look.IA_Look"))
  (:`Triggered`
    (`/Game/Game/player/components/BPC_Look.Look` (`self.BPC_Look`) ActionValue_X ActionValue_Y)))

(event `EnhancedInput|/Game/Settings/Input/IA_Jump`
  (params (ActionValue :type Boolean) (ElapsedSeconds :type "Float (double-precision)") (TriggeredSeconds :type "Float (double-precision)") (InputAction :type "InputAction Object Reference" :default "/Game/Settings/Input/IA_Jump.IA_Jump"))
  (:`Triggered`
    (`self.Jump`))
  (:`Canceled`
    (`self.StopJumping`)))

(fn `GetPlayer`
  (returns (player :type "/Game/Game/player/BP_PlayerCharacter Object Reference"))
  (return self))

(fn `UserConstructionScript`)
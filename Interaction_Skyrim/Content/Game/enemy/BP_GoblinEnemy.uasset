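; BP_GoblinEnemy is a goblin enemy that chases the player, can be burnt to death, and has an attack montage.
; From BeginPlay it runs AI MoveTo toward the player, repeating two seconds after each success but not on failure.
; A pause event from the player controller toggles its walk speed between zero and normal.
; GetBurnt activates a Niagara effect and destroys the goblin after a timer; Attack is not called within this graph.
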(event `self.ReceiveBeginPlay`
  (bind _playercontroller (message `/Game/Game/player/interface/BPI_Controller.GetController` (`GameplayStatics.GetPlayerController` 0)))
  (add `/Game/Settings/BP_PlayerController.SendOnPause` _playercontroller (delegate `MovementCancel`))
  (`self.ChasePlayer`))

(event `MovementCancel`
  (params (isPaused :type Boolean))
  (bind _charactermovement (`self.CharacterMovement`))
  (if isPaused
    (set `CharacterMovementComponent.MaxWalkSpeed` 0.0 _charactermovement)
    (else
      (set `CharacterMovementComponent.MaxWalkSpeed` 250.0 _charactermovement))))

(event `GetBurnt`
  (`ActorComponent.Activate` (`self.Niagara`) false)
  (`KismetSystemLibrary.K2_SetTimerDelegate` (delegate `death`) 3.0))

(event `ChasePlayer`
  (`|AIMoveTo` self (0.0 0.0 0.0) (`GameplayStatics.GetPlayerCharacter` 0) 150.0
    (:`OnSuccess`
      (`KismetSystemLibrary.Delay` 2.0)
      (`self.ChasePlayer`))))

(event `death`
  (`self.K2_DestroyActor`))

(event `Attack`
  (`|PlayMontage` (`self.Mesh`)))

(fn `UserConstructionScript`)
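; World item pickup actor, configured by an ItemData asset, that the player can collect when in range.
; On BeginPlay it async-loads the item's mesh, passes the data to its widget, and binds PickUpItem to the player's OnPickup event.
; Sphere overlap with the player toggles the widget and CanPickUp.
; A valid pickup sends ItemData through the player controller to the UI, then destroys the actor.
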(event `self.ReceiveBeginPlay`
  ; Data Asset setup
  (bind _object (`|LoadAsset` (`/Game/Game/Items/Data/PDA_ItemData.StaticMesh` (`self.itemData`)))
    (:`then`
      (message `/Game/Game/UI/BPI_Widget.SendItemData` (`WidgetComponent.GetWidget` (`self.Widget`)) (`self.itemData`))
      ; This event is called from the player, communicates with the HUD through a controller call
      (bind _player (message `/Game/Game/player/interface/BPI_Player.GetPlayer` (`GameplayStatics.GetPlayerCharacter` 0)))
      (add `/Game/Game/player/BP_PlayerCharacter.On_Pickup` _player (delegate `PickUpItem`)))
    (:`Completed`
      (bind _asstatic_mesh (cast `StaticMesh` _object))
      (`StaticMeshComponent.SetStaticMesh` (`self.StaticMesh`) _asstatic_mesh))))

(event `PickUpItem`
  ; This event is called from the player, communicates with the HUD through a controller call
  (if (`self.canPickUp`)
    (bind _playercontroller (message `/Game/Game/player/interface/BPI_Controller.GetController` (`GameplayStatics.GetPlayerController` 0)))
    (`/Game/Settings/BP_PlayerController.SendToUIPickUp` _playercontroller (`self.itemData`))
    (`self.K2_DestroyActor`)))

(event `self.Sphere.OnComponentBeginOverlap`
  (params (OverlappedComponent :type "PrimitiveComponent Object Reference") (OtherActor :type "Actor Object Reference") (OtherComp :type "PrimitiveComponent Object Reference") (OtherBodyIndex :type Integer) (bFromSweep :type Boolean) (SweepResult :type "HitResult Structure (by ref)"))
  ; Show and Hide ScreenView Widget UI of the item
  (if (== OtherActor (`GameplayStatics.GetPlayerCharacter` 0))
    (message `/Game/Game/UI/BPI_Widget.SetWVisibility` (`WidgetComponent.GetWidget` (`self.Widget`)) true)
    (set `self.canPickUp` true)))

(event `self.Sphere.OnComponentEndOverlap`
  (params (OverlappedComponent :type "PrimitiveComponent Object Reference") (OtherActor :type "Actor Object Reference") (OtherComp :type "PrimitiveComponent Object Reference") (OtherBodyIndex :type Integer))
  ; Show and Hide ScreenView Widget UI of the item
  (if (== OtherActor (`GameplayStatics.GetPlayerCharacter` 0))
    (message `/Game/Game/UI/BPI_Widget.SetWVisibility` (`WidgetComponent.GetWidget` (`self.Widget`)) false)
    (set `self.canPickUp` false)))

(fn `UserConstructionScript`)
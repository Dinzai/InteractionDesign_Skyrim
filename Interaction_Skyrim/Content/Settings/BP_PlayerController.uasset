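; Player controller Blueprint that sets up input and the player HUD and broadcasts pause requests.
; On BeginPlay it adds the IM_Context Enhanced Input mapping, creates WD_PlayerHUD, adds it to the viewport and switches to game-only input.
; The IA_OpenMneu action calls the SendOnPause dispatcher, signalling pause rather than handling a widget the controller does not own.
; A GetController function returns the controller itself.
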(event `self.ReceiveBeginPlay`
  ; Since the player controller adds the widget to the screen, But does not own the widget
  (`EnhancedInputSubsystemInterface.AddMappingContext` (pcsubsystem `EnhancedInputLocalPlayerSubsystem` self) "/Game/Settings/Input/IM_Context.IM_Context" 0 (struct))
  (bind _returnvalue (`|CreateWidget` "/Game/Game/UI/WD_PlayerHUD.WD_PlayerHUD_C" self))
  (`UserWidget.AddToViewport` _returnvalue 0)
  (`WidgetBlueprintLibrary.SetInputMode_GameOnly` self))

(event `EnhancedInput|/Game/Settings/Input/IA_OpenMneu`
  (params (ActionValue :type Boolean) (ElapsedSeconds :type "Float (double-precision)") (TriggeredSeconds :type "Float (double-precision)") (InputAction :type "InputAction Object Reference" :default "/Game/Settings/Input/IA_OpenMneu.IA_OpenMneu"))
  ; Because we do not own the widget, we send a signal
  (:`Triggered`
    (`self.SendOnPause`)))

(fn `GetController`
  (returns (playerController :type "/Game/Settings/BP_PlayerController Object Reference"))
  (return self))

(fn `UserConstructionScript`)